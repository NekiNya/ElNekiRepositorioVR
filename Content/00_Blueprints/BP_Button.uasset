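; BP_Button is a physical push button that reacts to overlaps with a VRPawn.
; It stores the relative location of ButtonMain on BeginPlay as the rest position.
; A pawn overlapping Button_main moves ButtonMain slightly down its local Y axis via MoveComponentTo, and leaving the separate Box component moves it back.
; The Blueprint only handles this movement and triggers no other action.
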(event `self.ReceiveBeginPlay`
  ; Button Pos Init
  (set `self.Buttom_pos1` (`SceneComponent.RelativeLocation` (`self.Button_main`))))

(event `self.Button_main.OnComponentBeginOverlap`
  (params (OverlappedComponent :type "PrimitiveComponent Object Reference") (OtherActor :type "Actor Object Reference") (OtherComp :type "PrimitiveComponent Object Reference") (OtherBodyIndex :type Integer) (bFromSweep :type Boolean) (SweepResult :type "HitResult Structure (by ref)"))
  (bind (_buttom_pos1_x _buttom_pos1_y) (`KismetMathLibrary.BreakVector` (`self.Buttom_pos1`)))
  ; Button Push
  (cast `/Game/VRTemplate/Blueprints/VRPawn` OtherActor)
  (`KismetSystemLibrary.MoveComponentTo` (`self.Button_main`) (`KismetMathLibrary.MakeVector` 0.0 (- _buttom_pos1_y 2.0))))

(event `self.Box.OnComponentEndOverlap`
  (params (OverlappedComponent :type "PrimitiveComponent Object Reference") (OtherActor :type "Actor Object Reference") (OtherComp :type "PrimitiveComponent Object Reference") (OtherBodyIndex :type Integer))
  (bind (_buttom_pos1_x _buttom_pos1_y) (`KismetMathLibrary.BreakVector` (`self.Buttom_pos1`)))
  ; Button Init
  (cast `/Game/VRTemplate/Blueprints/VRPawn` OtherActor)
  (`KismetSystemLibrary.MoveComponentTo` (`self.Button_main`) (`KismetMathLibrary.MakeVector` 0.0 _buttom_pos1_y)))

(fn `UserConstructionScript`)